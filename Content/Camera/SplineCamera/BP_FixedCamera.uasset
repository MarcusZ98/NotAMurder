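; Spline-rail camera actor that takes over the view, with a blend, when the player enters its box, optionally returning it on exit.
; Each tick, the spring arm eases toward the spline point nearest the player and matches spline rotation, while the camera can track the player in yaw and/or pitch.
; Construction previews the camera along the spline and sets arm length.
; Logic passing camera references to the character is disconnected.
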(event `self.ReceiveTick`
  (params (DeltaSeconds :type "Float (single-precision)"))
  (bind _springarm (`self.SpringArm`))
  (bind (_returnvalue_roll _returnvalue_pitch _returnvalue_yaw) (`KismetMathLibrary.BreakRotator` (`SceneComponent.K2_GetComponentRotation` (`self.Camera`))))
  (bind (_returnvalue_roll_2 _returnvalue_pitch_2 _returnvalue_yaw_2) (`KismetMathLibrary.BreakRotator` (`KismetMathLibrary.FindLookAtRotation` (`SceneComponent.K2_GetComponentLocation` (`self.Camera`)) (`self.K2_GetActorLocation` (`GameplayStatics.GetPlayerCharacter` 0)))))
  (set `self.Delta Seconds` DeltaSeconds)
  ;[1 1 1] Sets the location for the spring arm so it follows the spline
  (`SceneComponent.K2_SetWorldLocation` (`self.SpringArm`) (`KismetMathLibrary.VInterpTo` (`SceneComponent.K2_GetComponentLocation` (`self.SpringArm`)) (`SplineComponent.FindLocationClosestToWorldLocation` (`self.Spline`) (`self.K2_GetActorLocation` (`GameplayStatics.GetPlayerCharacter` 0)) "World") (`self.Delta Seconds`) (`self.Interp Speed`)) false false)
  ;[1 1 1] Sets the rotation for the spring arm so it follows  the spline
  (`SceneComponent.K2_SetWorldRotation` _springarm (`KismetMathLibrary.RInterpTo` (`SceneComponent.K2_GetComponentRotation` _springarm) (`SplineComponent.FindRotationClosestToWorldLocation` (`self.Spline`) (`SceneComponent.K2_GetComponentLocation` (`self.SpringArm`)) "World") (`self.Delta Seconds`) (`self.Interp Speed`)) false false)
  ;[1 1 1] Roatates the camera of the spring arm to follow the player in selected Axis
  (if (or (`self.HorizonatlPlayerFollow`) (`self.VerticatlPlayerFollow`))
    (`SceneComponent.K2_SetWorldRotation` (`self.Camera`) (`KismetMathLibrary.RInterpTo` (`SceneComponent.K2_GetComponentRotation` (`self.Camera`)) (`KismetMathLibrary.MakeRotator` _returnvalue_roll (select `bool` (`self.VerticatlPlayerFollow`) :`false` _returnvalue_pitch :`true` _returnvalue_pitch_2) (select `bool` (`self.HorizonatlPlayerFollow`) :`false` _returnvalue_yaw :`true` _returnvalue_yaw_2)) (`self.Delta Seconds`) (`self.Interp Speed`)) false false)))

(event `self.Box.OnComponentBeginOverlap`
  (params (OverlappedComponent :type "PrimitiveComponent Object Reference") (OtherActor :type "Actor Object Reference") (OtherComp :type "PrimitiveComponent Object Reference") (OtherBodyIndex :type Integer) (bFromSweep :type Boolean) (SweepResult :type "HitResult Structure (by ref)"))
  ;[1 1 1] Changes the camera view to this BP camera
  (if (== OtherActor (`GameplayStatics.GetPlayerCharacter` 0))
    (set `self.IsPlayerInside` true)
    (`PlayerController.SetViewTargetWithBlend` (`GameplayStatics.GetPlayerController` 0) self (`self.Blend Time`) (`self.Blend Func`) 2.0 true)))

(event `self.Box.OnComponentEndOverlap`
  (params (OverlappedComponent :type "PrimitiveComponent Object Reference") (OtherActor :type "Actor Object Reference") (OtherComp :type "PrimitiveComponent Object Reference") (OtherBodyIndex :type Integer))
  ;[1 1 1] Changes back the camera view to the players lokal camera
  (if (== OtherActor (`GameplayStatics.GetPlayerCharacter` 0))
    (set `self.IsPlayerInside` false)
    (if (`self.ChangeOnExit`)
      (`PlayerController.SetViewTargetWithBlend` (`GameplayStatics.GetPlayerController` 0) (`GameplayStatics.GetPlayerCharacter` 0) 3.0 "VTBlend_EaseInOut" 2.0 true))))

(fn `OnFIxedCamEndOverlap`)

(fn `OnFixedCamOverlap`
  (`PlayerController.SetViewTargetWithBlend` (`GameplayStatics.GetPlayerController` 0) self (`self.Blend Time`) (`self.Blend Func`) 2.0 true))

(fn `Set Player Collision Offset`
  (set `self.PlayerCollisionOffset` (select `bool` (> (`KismetMathLibrary.Dot_VectorVector` (`SceneComponent.GetForwardVector` (`self.Camera`)) (`self.GetActorForwardVector` (`GameplayStatics.GetPlayerCharacter` 0))) 0.0) :`false` (`self.PlayerFrontCollisionOffset`) :`true` (`self.PlayerBackCollisionOffset`))))

(fn `SnapToSpline`
  (bind _returnvalue (`KismetMathLibrary.Lerp` 0.0 (`SplineComponent.GetSplineLength` (`self.Spline`)) (`self.CameraPoint`)))
  (`SceneComponent.K2_SetWorldTransform` (`self.Camera`) (`KismetMathLibrary.MakeTransform` (`SplineComponent.GetLocationAtDistanceAlongSpline` (`self.Spline`) _returnvalue "World") (`SplineComponent.GetRotationAtDistanceAlongSpline` (`self.Spline`) _returnvalue "World")) false false))

(fn `UserConstructionScript`
  (`self.SnapToSpline`)
  (set `SpringArmComponent.TargetArmLength` (`self.SpringArmLenght`) (`self.SpringArm`)))