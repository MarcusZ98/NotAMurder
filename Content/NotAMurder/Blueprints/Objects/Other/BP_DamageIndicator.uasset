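; BP_DamageIndicator is a short-lived world actor that displays a damage number through a WB_DamageIndicator widget component.
; On BeginPlay it passes Damage to the widget and computes a randomized end point up and to the right using the player's vectors.
; A timeline sets its location each update, then destroys it on finish.
; The lerp uses StartPOS at both ends, leaving EndPOS unused, so the actor stays in place.
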(event `self.ReceiveBeginPlay`
  (bind _aswb_damage_indicator (cast `/Game/NotAMurder/Blueprints/Widgets/WB_DamageIndicator` (`WidgetComponent.GetWidget` (`self.Widget`))))
  (`/Game/NotAMurder/Blueprints/Widgets/WB_DamageIndicator.Set Damage` _aswb_damage_indicator (`self.Damage`))
  (bind _output_get (set `self.Start POS` (`self.K2_GetActorLocation`)))
  (bind _asbp_player (cast `/Game/NotAMurder/Blueprints/Characters/Player/BP_Player` (`GameplayStatics.GetPlayerCharacter` 0)))
  (bind (_up_vector _right_vector) (`/Game/NotAMurder/Blueprints/Characters/Player/BP_Player.Get Vectors` _asbp_player))
  (set `self.End POS` (+ _output_get (* _up_vector (`KismetMathLibrary.RandomFloatInRange` 40.0 50.0)) (* _right_vector (`KismetMathLibrary.RandomFloatInRange` 20.0 30.0))))
  (bind (_direction _newtrack_0) (`Timeline|Timeline`)
    (:`Update`
      (`self.K2_SetActorLocation` (`KismetMathLibrary.VLerp` (`self.Start POS`) (`self.Start POS`) _newtrack_0)))
    (:`Finished`
      (`self.K2_DestroyActor`))))

(fn `UserConstructionScript`)