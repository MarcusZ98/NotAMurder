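; BP_Projectile_LargeOrb is a child projectile Blueprint for a large orb fired by a weapon.
; On BeginPlay it runs parent logic, then rescales its velocity to the projectile speed in the instigator's weapon data, keeping direction.
; Each Tick it looks up the player via GetActorOfClass and destroys itself once it is behind the player's facing, using a dot product, and beyond a fixed distance.
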(event `self.ReceiveBeginPlay`
  (`parent.ReceiveBeginPlay`)
  (bind _returnvalue (message `Character_Interface.GetCharacterData` (`self.GetInstigator`)))
  (bind (_weapondata_damagepershot _weapondata_firerate _weapondata_projectile _weapondata_projectilespeed) (break `WeaponData` (`BaseWeapon.WeaponData` (`.WeaponInstance` (break `CharacterData` _returnvalue)))))
  (set `MovementComponent.Velocity` (* (`KismetMathLibrary.Normal` (`MovementComponent.Velocity` (`self.ProjectileMovement`))) _weapondata_projectilespeed) (`self.ProjectileMovement`)))

(event `self.ReceiveTick`
  (params (DeltaSeconds :type "Float (single-precision)"))
  (bind _returnvalue (`self.K2_GetActorLocation`))
  (bind _returnvalue_2 (`GameplayStatics.GetActorOfClass` "/Game/NotAMurder/Blueprints/Characters/Player/BP_PlayerParent1.BP_PlayerParent1_C"))
  (bind _returnvalue_3 (`self.K2_GetActorLocation` _returnvalue_2))
  (if (and (< (`KismetMathLibrary.Dot_VectorVector` (`self.GetActorForwardVector` _returnvalue_2) (- _returnvalue _returnvalue_3)) 0.0) (> (`KismetMathLibrary.Vector_Distance` _returnvalue_3 _returnvalue) 500.0))
    (`self.K2_DestroyActor`)))

(fn `UserConstructionScript`
  (`parent.UserConstructionScript`))