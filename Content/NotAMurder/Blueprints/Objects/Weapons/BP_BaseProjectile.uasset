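; Base projectile for weapons that damages characters of a different type than its instigator and expires after a set lifetime.
; ProjectileData supplies the lifetime and the movement's max speed.
; On sphere overlap, character types are compared through interface messages to filter targets.
; Damage multiplies the owning weapon's per-shot damage by the instigator's multiplier, then a Niagara hit effect spawns and the projectile is destroyed.
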(event `self.ReceiveBeginPlay`
  ;[0.6764 1 0.6936] Destroy Projectile after set amount of time
  (`KismetSystemLibrary.Delay` (`.ProjectileLife` (break `ProjectileData` (`self.ProjectileData`))))
  (`self.K2_DestroyActor`))

(event `self.Sphere.OnComponentBeginOverlap`
  (params (OverlappedComponent :type "PrimitiveComponent Object Reference") (OtherActor :type "Actor Object Reference") (OtherComp :type "PrimitiveComponent Object Reference") (OtherBodyIndex :type Integer) (bFromSweep :type Boolean) (SweepResult :type "HitResult Structure (by ref)"))
  (bind _result (`self.IsDifferentCharacter?` OtherActor))
  (if _result
    (bind _damage (`self.HowMuchDamageToDeal?` (`self.GetInstigator`)))
    (`GameplayStatics.ApplyDamage` OtherActor _damage null (`self.GetInstigator`))
    (`NiagaraFunctionLibrary.SpawnSystemAtLocation` "/Game/ProjectileHitVFX/NS/NS_Hit_HolyWind.NS_Hit_HolyWind" SweepResult_ImpactPoint)
    (`self.K2_DestroyActor`)))

(fn `HowMuchDamageToDeal?`
  (params (Instigator :type "Actor Object Reference"))
  (returns (Damage :type "Float (double-precision)"))
  (locals (`TEMP FLOAT` :type "Float (double-precision)" :default 65.0))
  (bind _returnvalue (message `Character_Interface.GetCharacterData` Instigator))
  (bind _asbase_weapon (cast `BaseWeapon` (`self.GetOwner`)))
  (return (* (`.DamagePerShot` (break `WeaponData` (`BaseWeapon.WeaponData` _asbase_weapon))) (`.DamageMultiplier` (break `CharacterData` _returnvalue)))))

(fn `IsDifferentCharacter?`
  (params (`Other Actor` :type "Actor Object Reference"))
  (returns (Result :type Boolean))
  (bind _returnvalue (`self.GetInstigator`))
  (bind _returnvalue_2 (message `Character_Interface.GetCharacterType` `Other Actor`))
  (`/Engine/EditorBlueprintResources/StandardMacros.IsValid` _returnvalue
    (:`Is Valid`
      (bind _returnvalue_3 (message `Character_Interface.GetCharacterType` _returnvalue))
      (return (`|EnumInequality` _returnvalue_3 _returnvalue_2)))))

(fn `UserConstructionScript`
  (set `ProjectileMovementComponent.MaxSpeed` (`.ProjectileSpeed` (break `ProjectileData` (`self.ProjectileData`))) (`self.ProjectileMovement`)))