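; Camera actor that becomes the view target on BeginPlay, pairing a cursor-steered camera with an input-moved child actor.
; Each tick, mouse offsets beyond screen-center limits nudge camera yaw and pitch through RInterpTo, clamped to narrow angles.
; IA_Move input shifts the child actor along local Y and Z.
; SpeedableInterface edits MovementSpeed, which Tick ignores in favor of Speed; cursor-follow and aiming experiments are disconnected.
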(event `self.ReceiveBeginPlay`
  (bind (_relativerotation_roll _relativerotation_pitch _relativerotation_yaw) (`KismetMathLibrary.BreakRotator` (`SceneComponent.RelativeRotation` (`self.Camera`))))
  (`PlayerController.SetViewTargetWithBlend` (`GameplayStatics.GetPlayerController` 0) self 0.0 "VTBlend_Linear" 0.0 false)
  (set `self.NewRollValue` _relativerotation_roll)
  (set `self.NewPitchValue` _relativerotation_pitch)
  (set `self.NewYawValue` _relativerotation_yaw)
  (set `self.OriginalMovementSpeed` (`self.Speed`)))

(event `self.ReceiveTick`
  (params (DeltaSeconds :type "Float (single-precision)"))
  (bind (_returnvalue_x _returnvalue_y) (`KismetMathLibrary.BreakVector2D` (`WidgetLayoutLibrary.GetViewportSize`)))
  (bind (_returnvalue_x_2 _returnvalue_y_2) (`KismetMathLibrary.BreakVector2D` (`|GetInputActionValue`)))
  (bind _returnvalue (* DeltaSeconds 0.8))
  (bind _childactor (`self.ChildActor`))
  (bind (_locationx _locationy) (`PlayerController.GetMousePosition` (`GameplayStatics.GetPlayerController` 0)))
  (bind (_relativerotation_roll _relativerotation_pitch _relativerotation_yaw) (`KismetMathLibrary.BreakRotator` (`SceneComponent.RelativeRotation` (`self.Camera`))))
  (bind (_relativerotation_roll_2 _relativerotation_pitch_2 _relativerotation_yaw_2) (`KismetMathLibrary.BreakRotator` (`SceneComponent.RelativeRotation` (`self.Camera`))))
  (bind (_relativelocation_x _relativelocation_y _relativelocation_z) (`KismetMathLibrary.BreakVector` (`SceneComponent.RelativeLocation` _childactor)))
  (bind _returnvalue_2 (- _locationy (/ _returnvalue_y 2.0)))
  (bind _returnvalue_3 (- _locationx (/ _returnvalue_x 2.0)))
  (bind (_returnvalue_roll _returnvalue_pitch _returnvalue_yaw) (`KismetMathLibrary.BreakRotator` (`KismetMathLibrary.RInterpTo` (`SceneComponent.RelativeRotation` (`self.Camera`)) (`KismetMathLibrary.MakeRotator` _relativerotation_roll_2 (`self.NewPitchValue`) (`self.NewYawValue`)) (* DeltaSeconds (`self.Speed`)) 1.0)))
  (`|ExecutionSequence`
    (:`then_0`
      (if (> (`KismetMathLibrary.Abs` _returnvalue_3) (`self.HorizontalLimit`))
        (set `self.NewYawValue` (+ _relativerotation_yaw (* (`KismetMathLibrary.SignOfFloat` _returnvalue_3) 100.0)))
        (else
          (set `self.NewYawValue` _relativerotation_yaw_2))))
    (:`then_1`
      (if (> (`KismetMathLibrary.Abs` _returnvalue_2) (`self.VerticalLimit`))
        (set `self.NewPitchValue` (+ (* (`KismetMathLibrary.SignOfFloat` _returnvalue_2) -100.0) _relativerotation_pitch))
        (else
          (set `self.NewPitchValue` _relativerotation_pitch_2))))
    (:`then_2`
      (`SceneComponent.K2_SetRelativeRotation` (`self.Camera`) (`KismetMathLibrary.MakeRotator` (`KismetMathLibrary.FClamp` _returnvalue_roll -5.0 5.0) (`KismetMathLibrary.FClamp` _returnvalue_pitch -10.0 10.0) (`KismetMathLibrary.FClamp` _returnvalue_yaw -20.0 20.0)) false false))
    (:`then_3`
      (`SceneComponent.K2_SetRelativeLocation` _childactor (`KismetMathLibrary.MakeVector` _relativelocation_x (`KismetMathLibrary.Lerp` _relativelocation_y (+ _relativelocation_y (* _returnvalue_x_2 500.0)) _returnvalue) (`KismetMathLibrary.Lerp` _relativelocation_z (+ _relativelocation_z (* _returnvalue_y_2 500.0)) _returnvalue)) false false))))

(event `self.SetSpeed`
  (params (NewSpeed :type "Float (single-precision)"))
  ;[1 1 1] SpeedableInterface
  (set `self.MovementSpeed` NewSpeed))

(event `self.ResetSpeed`
  ;[1 1 1] SpeedableInterface
  (set `self.MovementSpeed` (`self.OriginalMovementSpeed`)))

(event `self.MultiplySpeed`
  (params (Multiplier :type "Float (single-precision)"))
  ;[1 1 1] SpeedableInterface
  (set `self.MovementSpeed` (* Multiplier (`self.MovementSpeed`))))

(fn `GetSpeed`
  (returns (ReturnValue :type "Float (single-precision)"))
  (return (`self.MovementSpeed`)))

(fn `MoveChildrenLocal`
  (params (NewY :type "Float (double-precision)") (DeltaTime :type "Float (double-precision)"))
  (returns (newYValue :type "Float (double-precision)"))
  (return 0.0))

(fn `UserConstructionScript`)