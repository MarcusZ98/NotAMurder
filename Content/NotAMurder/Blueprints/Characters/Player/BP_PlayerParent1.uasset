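; Player camera rig that becomes the view target and carries BP_Player as a child actor for cursor-aimed play against enemies.
; Each tick, the cursor nearing screen edges turns the clamped camera, whose angles shift the movement bounds via tangent times arm length.
; IA_Move slides the player on local Y/Z within those bounds.
; A sphere trace blends cursor sensitivity for aim assist, while a line trace switches the HUD cursor's enemy focus.
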(event `self.ReceiveBeginPlay`
  (bind (_returnvalue_x _returnvalue_y) (`KismetMathLibrary.BreakVector2D` (/ (`WidgetLayoutLibrary.GetViewportSize`) (2.0 2.0))))
  ;[1 1 1] Sets this camera as view
  (`PlayerController.SetViewTargetWithBlend` (`GameplayStatics.GetPlayerController` 0) self 0.0 "VTBlend_Linear" 0.0 false)
  ;[1 1 1] Sets initial center XY position
  (set `self.CenterPositionX` _returnvalue_x)
  (set `self.CenterPositionY` _returnvalue_y)
  ;[1 1 1] BOx that represents player movement limits
  (`BoxComponent.SetBoxExtent` (`self.Box`) (`KismetMathLibrary.MakeVector` 50.0 (`self.InitialPlayerPositionRightLimitX`) (`self.InitialPlayerPositionUpperLimitY`)) true)
  (set `PlayerController.bEnableMouseOverEvents` true (`GameplayStatics.GetPlayerController` 0))
  ;[1 1 1] Sets cursor widget variable
  (`KismetSystemLibrary.DelayUntilNextTick`)
  (bind _asplayer_hud (cast `/Game/NotAMurder/Blueprints/Widgets/Player_HUD` (`PlayerController.GetHUD` (`GameplayStatics.GetPlayerController` 0))))
  (set `self.CursorWidget` (`/Game/NotAMurder/Blueprints/Widgets/Player_HUD.CursorWidget` _asplayer_hud))
  (set `self.InitialArmLength` (`SpringArmComponent.TargetArmLength` (`self.SpringArm`))))

(event `self.ReceiveTick`
  (params (DeltaSeconds :type "Float (single-precision)"))
  (bind _returnvalue (`GameplayStatics.GetPlayerController` 0))
  (bind (_returnvalue_x _returnvalue_y) (`KismetMathLibrary.BreakVector2D` (`WidgetLayoutLibrary.GetViewportSize`)))
  (bind (_returnvalue_x_2 _returnvalue_y_2) (`KismetMathLibrary.BreakVector2D` (`|GetInputActionValue`)))
  (bind _rotationlimityaw (`self.RotationLimitYaw`))
  (bind _rotationlimitpitch (`self.RotationLimitPitch`))
  (bind (_locationx _locationy) (`PlayerController.GetMousePosition` _returnvalue))
  (bind (_locationx_2 _locationy_2) (`PlayerController.GetMousePosition` (`GameplayStatics.GetPlayerController` 0)))
  (bind (_returnvalue_x_3 _returnvalue_y_3) (`KismetMathLibrary.BreakVector2D` (/ (`WidgetLayoutLibrary.GetViewportSize`) (2.0 2.0))))
  (bind _childactor (`ChildActorComponent.ChildActor` (`self.ChildActor`)))
  (bind (_relativerotation_roll _relativerotation_pitch _relativerotation_yaw) (`KismetMathLibrary.BreakRotator` (`SceneComponent.RelativeRotation` (`self.Camera`))))
  (bind (_relativelocation_x _relativelocation_y _relativelocation_z) (`KismetMathLibrary.BreakVector` (`SceneComponent.RelativeLocation` (`self.ChildActor`))))
  (bind _relativelocation_x_2 (`KismetMathLibrary.BreakVector` (`SceneComponent.RelativeLocation` (`self.ChildActor`))))
  (bind (_relativerotation_roll_2 _relativerotation_pitch_2 _relativerotation_yaw_2) (`KismetMathLibrary.BreakRotator` (`SceneComponent.RelativeRotation` (`self.Camera`))))
  (bind (_relativerotation_roll_3 _relativerotation_pitch_3 _relativerotation_yaw_3) (`KismetMathLibrary.BreakRotator` (`SceneComponent.RelativeRotation` (`self.Box`))))
  (bind (_relativerotation_roll_4 _relativerotation_pitch_4) (`KismetMathLibrary.BreakRotator` (`SceneComponent.RelativeRotation` (`self.Camera`))))
  (bind (_relativerotation_roll_5 _relativerotation_pitch_5 _relativerotation_yaw_4) (`KismetMathLibrary.BreakRotator` (`SceneComponent.RelativeRotation` (`self.Camera`))))
  (bind _worldposition (`GameplayStatics.DeprojectScreenToWorld` (`GameplayStatics.GetPlayerController` 0) (`KismetMathLibrary.MakeVector2D` (/ _returnvalue_x 2.0) (/ _returnvalue_y 2.0))))
  (bind _array (`|MakeArray` self (`ChildActorComponent.ChildActor` (`self.ChildActor`)) :!type "Actor Object Reference"))
  (bind _returnvalue_2 (* (`KismetMathLibrary.DegTan` (`self.RotationLimitPitch`)) (`self.InitialArmLength`)))
  (bind _returnvalue_3 (* (`KismetMathLibrary.DegTan` (`self.RotationLimitPitch`)) (`self.InitialArmLength`)))
  (bind (_returnvalue_roll _returnvalue_pitch _returnvalue_yaw) (`KismetMathLibrary.BreakRotator` (`KismetMathLibrary.RLerp` (`KismetMathLibrary.MakeRotator` _relativerotation_roll_2 _relativerotation_pitch_2 _relativerotation_yaw_2) (`KismetMathLibrary.MakeRotator` 0.0 (`KismetMathLibrary.FClamp` (`self.TargetPitchValue`) -179.0 179.0) (`KismetMathLibrary.FClamp` (`self.TargetYawValue`) -179.0 179.0)) (* (`self.Delta Seconds`) (`self.RotationForce`)))))
  (bind _returnvalue_4 (* (`KismetMathLibrary.DegTan` _relativerotation_yaw) (`self.InitialArmLength`)))
  (bind _returnvalue_5 (+ (`self.InitialPlayerPositionRightLimitX`) _returnvalue_2))
  (bind _returnvalue_6 (- (* (`self.InitialPlayerPositionRightLimitX`) -1.0) _returnvalue_2))
  (bind _returnvalue_7 (* (`KismetMathLibrary.DegTan` _relativerotation_pitch_4) (`self.InitialArmLength`)))
  (bind _returnvalue_8 (+ (`self.InitialPlayerPositionUpperLimitY`) _returnvalue_3))
  (bind _returnvalue_9 (- (* (`self.InitialPlayerPositionUpperLimitY`) -1.0) _returnvalue_3))
  (bind (_returnvalue_x_4 _returnvalue_y_4 _returnvalue_z) (`KismetMathLibrary.BreakVector` (`KismetMathLibrary.VLerp` (`SceneComponent.RelativeLocation` (`self.ChildActor`)) (`KismetMathLibrary.MakeVector` _relativelocation_x_2 (`KismetMathLibrary.FClamp` (+ (* _returnvalue_x_2 1000.0) _relativelocation_y) (`self.PlayerPositionLeftLimitX`) (`self.PlayerPositionRightLimitX`)) (`KismetMathLibrary.FClamp` (+ _relativelocation_z (* _returnvalue_y_2 1000.0)) (`self.PlayerPositionLowerLimitY`) (`self.PlayerPositionUpperLimitY`))) (* (`self.Delta Seconds`) (`self.MovementForce`)))))
  (bind _returnvalue_10 (+ _worldposition (* (`.WorldDirection` (`GameplayStatics.DeprojectScreenToWorld` _returnvalue (`KismetMathLibrary.MakeVector2D` _locationx _locationy))) (25000.0 25000.0 25000.0))))
  (set `self.Delta Seconds` DeltaSeconds)
  ;[1 1 1] Sets center position XY
  (set `self.CenterPositionY` _returnvalue_x_3)
  (set `self.CenterPositionY` _returnvalue_y_3)
  (`|ExecutionSequence`
    (:`then_0`
      ;[1 1 1] TracksCursor position
      (bind _output_get (set `self.DeltaX` (- _locationx_2 (`self.CenterPositionX`))))
      (set `self.DistanceScaleX` (/ _output_get (`self.CenterPositionX`))))
    (:`then_1`
      (bind _output_get_2 (set `self.DeltaY` (- _locationy_2 (`self.CenterPositionY`))))
      (set `self.DistanceScaleY` (/ _output_get_2 (`self.CenterPositionY`))))
    (:`then_2`
      ;[1 1 1] Checks if cursor is outside the limits
      (if (> (`KismetMathLibrary.Abs` (`self.DistanceScaleX`)) (`self.HorizontalLimitBR`))
        (set `self.TargetYawValue` (+ (* (`KismetMathLibrary.SignOfFloat` (`self.DeltaX`)) 50.0) _relativerotation_yaw_4))
        (else
          (set `self.TargetYawValue` _relativerotation_yaw_4))))
    (:`then_3`
      (if (> (`KismetMathLibrary.Abs` (`self.DistanceScaleY`)) (`self.VerticalLimitBR`))
        (set `self.TargetPitchValue` (+ (* (`KismetMathLibrary.SignOfFloat` (`self.DeltaY`)) -50.0) _relativerotation_pitch_5))
        (else
          (set `self.TargetPitchValue` _relativerotation_pitch_5))))
    (:`then_4`
      ;[1 1 1] Sets new camera rotation
      (`SceneComponent.K2_SetRelativeRotation` (`self.Camera`) (`KismetMathLibrary.MakeRotator` 0.0 (`KismetMathLibrary.FClamp` _returnvalue_pitch (* _rotationlimitpitch -1.0) _rotationlimitpitch) (`KismetMathLibrary.FClamp` _returnvalue_yaw (* _rotationlimityaw -1.0) _rotationlimityaw)) false false))
    (:`then_5`
      ;[1 1 1] Calculates new player movvement limits
      ;;[1 1 1] Sets new location for the box representing the player movement limits
      (`SceneComponent.K2_SetRelativeLocation` (`self.Box`) (`KismetMathLibrary.MakeVector` _relativerotation_roll_3 (+ _relativerotation_pitch_3 _returnvalue_4) (+ _relativerotation_yaw_3 _returnvalue_7)) false false)
      ;;[1 1 1] Sets new movement limits
      (set `self.PlayerPositionUpperLimitY` (`KismetMathLibrary.FClamp` (+ (`self.InitialPlayerPositionUpperLimitY`) _returnvalue_7) _returnvalue_9 _returnvalue_8))
      (set `self.PlayerPositionLowerLimitY` (`KismetMathLibrary.FClamp` (+ -130.0 (* (`self.InitialPlayerPositionUpperLimitY`) -1.0)) _returnvalue_9 _returnvalue_8))
      (set `self.PlayerPositionLeftLimitX` (`KismetMathLibrary.FClamp` (+ (* (`self.InitialPlayerPositionRightLimitX`) -1.0) _returnvalue_4) _returnvalue_6 _returnvalue_5))
      (set `self.PlayerPositionRightLimitX` (`KismetMathLibrary.FClamp` (+ _returnvalue_4 (`self.InitialPlayerPositionRightLimitX`)) _returnvalue_6 _returnvalue_5)))
    (:`then_6`
      ;[1 1 1] Moves the actor child localy in only two axis
      (`SceneComponent.K2_SetRelativeLocation` (`self.ChildActor`) (`KismetMathLibrary.MakeVector` _returnvalue_x_4 _returnvalue_y_4 _returnvalue_z) false false))
    (:`then_7`
      ;[1 1 1] LineTrace looking for enemies
      (bind _outhit (`KismetSystemLibrary.SphereTraceSingle` _worldposition _returnvalue_10 (`self.AimAssist radius`) "TraceTypeQuery1" false _array (`self.Draw Debug Type`)))
      (if (`KismetSystemLibrary.DoesImplementInterface` (`.HitActor` (`GameplayStatics.BreakHitResult` _outhit)) "/Script/NotAMurder.Enemy_Interface")
        (bind _asbp_player (cast `/Game/NotAMurder/Blueprints/Characters/Player/BP_Player` _childactor))
        (set `/Game/NotAMurder/Blueprints/Characters/Player/BP_Player.CursorSensitivity` (`KismetMathLibrary.Lerp` (`/Game/NotAMurder/Blueprints/Characters/Player/BP_Player.CursorSensitivity` _asbp_player) (`self.CursorSensitivityOnEnemies`) (* (`self.Delta Seconds`) 20.0)) _asbp_player)
        (else
          (bind _asbp_player_2 (cast `/Game/NotAMurder/Blueprints/Characters/Player/BP_Player` _childactor))
          (set `/Game/NotAMurder/Blueprints/Characters/Player/BP_Player.CursorSensitivity` (`KismetMathLibrary.Lerp` (`/Game/NotAMurder/Blueprints/Characters/Player/BP_Player.CursorSensitivity` _asbp_player_2) (`self.CursorSensitivityOnDefault`) (* (`self.Delta Seconds`) 10.0)) _asbp_player_2)))
      (bind _outhit_2 (`KismetSystemLibrary.LineTraceSingle` _worldposition _returnvalue_10 "TraceTypeQuery1" false _array (`self.Draw Debug Type`) false))
      (if (`KismetSystemLibrary.DoesImplementInterface` (`.HitActor` (`GameplayStatics.BreakHitResult` _outhit_2)) "/Script/NotAMurder.Enemy_Interface")
        (`/Game/NotAMurder/Blueprints/Widgets/BP_Crosshair.OnEnemyFocus` (`self.CursorWidget`))
        (else
          (`/Game/NotAMurder/Blueprints/Widgets/BP_Crosshair.OnDeafultFocus` (`self.CursorWidget`)))))))

(fn `MoveChildrenLocal`
  (params (NewY :type "Float (double-precision)") (DeltaTime :type "Float (double-precision)"))
  (returns (newYValue :type "Float (double-precision)"))
  (return 0.0))

(fn `UserConstructionScript`)