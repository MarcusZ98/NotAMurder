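; Spline path actor that moves a referenced actor along its spline in an endless loop, facing it along the spline tangent.
; The construction script snaps that actor to the first spline point.
; On BeginPlay a timeline drives distance from start to last point, then restarts from the beginning when finished.
; Its play rate is the inverse of MovementSpeed, so higher values mean slower travel.
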(event `self.ReceiveTick`
  (params (DeltaSeconds :type "Float (single-precision)")))

(event `self.ReceiveBeginPlay`
  (`TimelineComponent.SetPlayRate` (`self.Timeline`) (/ 1.0 (`self.MovementSpeed`)))
  (`self.Play Timeline`))

(event `Play Timeline`
  (bind _spline (`self.Spline`))
  (bind _spline_2 (`self.Spline`))
  (bind (_direction _alpha) (`Timeline|Timeline` :!via `PlayFromStart`)
    (:`Update`
      (bind _returnvalue (`KismetMathLibrary.Lerp` 0.0 (`SplineComponent.GetDistanceAlongSplineAtSplinePoint` _spline (- (`SplineComponent.GetNumberOfSplinePoints` _spline) 1)) _alpha))
      (`self.K2_SetActorLocationAndRotation` (`self.ActorToMove`) (`SplineComponent.GetLocationAtDistanceAlongSpline` _spline_2 _returnvalue "World") (`KismetMathLibrary.Conv_VectorToRotator` (`SplineComponent.GetTangentAtDistanceAlongSpline` _spline_2 _returnvalue "World")) false false))
    (:`Finished`
      (`self.Play Timeline`))))

(fn `UserConstructionScript`
  (`self.K2_SetActorLocation` (`self.ActorToMove`) (`SplineComponent.GetLocationAtSplinePoint` (`self.Spline`) 0 "World") false false))