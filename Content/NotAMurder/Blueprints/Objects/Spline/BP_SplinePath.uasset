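; Spline path actor that carries either the player or an enemy group along its spline.
; Each tick advances distance by the character's current speed, then moves the player parent or enemy leader there.
; Construction snaps the player to the start or lays out enemy spawn markers in a grid.
; BeginPlay starts player movement, or spawns a hidden enemy leader with attached followers and optional data overrides.
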(event `Stop Spline`
  (`self.SetActorTickEnabled` false))

(event `Start Spline`
  (`self.SetActorTickEnabled` true))

(event `self.ReceiveBeginPlay`
  (switch `ECharacterType` (`self.CharacterType`)
    (:`Player`
      (`self.AttachPlayerToSpline`)
      (`self.Start Spline`))
    (:`Enemy`
      (`self.AttachEnemyToSpline`))))

(event `self.ReceiveTick`
  (params (DeltaSeconds :type "Float (single-precision)"))
  (switch `ECharacterType` (`self.CharacterType`)
    (:`Player`
      (`self.MovePlayerAlongSpline` DeltaSeconds))
    (:`Enemy`
      (`self.MoveEnemiesAlongSpline` DeltaSeconds))))

(fn `AttachEnemyToSpline`
  (bind _returnvalue (`|SpawnActorFromClass` (`self.EnemyClass`) (`SceneComponent.K2_GetComponentToWorld` (`self.Root`)) "AlwaysSpawn" "MultiplyWithRoot" null null))
  (bind _output_get (set `self.EnemyParent` _returnvalue))
  (if (`self.bOverrideCharacterData`)
    (message `Character_Interface.SetCharacterData` _output_get (`self.OverridenCharacterData`))
    (if (`self.bOverrideEnemyData`)
      (message `Enemy_Interface.SetEnemyData` _output_get (`self.OverriddenEnemyData`))))
  (`self.SetActorHiddenInGame` _output_get true)
  (for _array_element (`self.EnemySpawnPonts`)
    (bind _returnvalue_2 (`|SpawnActorFromClass` (`self.EnemyClass`) (`SceneComponent.K2_GetComponentToWorld` _array_element) "AlwaysSpawn" "MultiplyWithRoot" null null))
    (if (`self.bOverrideEnemyData`)
      (message `Enemy_Interface.SetEnemyData` _returnvalue_2 (`self.OverriddenEnemyData`))
      (if (`self.bOverrideCharacterData`)
        (message `Character_Interface.SetCharacterData` _returnvalue_2 (`self.OverridenCharacterData`))))
    (`self.K2_AttachToActor` _returnvalue_2 (`self.EnemyParent`) "None" "KeepWorld" "KeepRelative" "KeepRelative" true))
  (return))

(fn `AttachPlayerToSpline`
  (bind _asbp_player_parent_1 (cast `/Game/NotAMurder/Blueprints/Characters/Player/BP_PlayerParent1` (`self.PlayerParent`)))
  (bind _asbp_player (cast `/Game/NotAMurder/Blueprints/Characters/Player/BP_Player` (`ChildActorComponent.ChildActor` (`/Game/NotAMurder/Blueprints/Characters/Player/BP_PlayerParent1.ChildActor` _asbp_player_parent_1))))
  (set `self.PlayerCharacter` _asbp_player)
  (if (not (`self.bOverrideCharacterData`))
    (`self.K2_SetActorTransform` (`self.PlayerParent`) (`SplineComponent.GetTransformAtSplinePoint` (`self.SplineComponent`) 0 "World" false) false false)))

(fn `MoveActorAlongSpline`
  (params (ActorToMove :type "Actor Object Reference") (Delta :type "Float (double-precision)"))
  (bind (_returnvalue_location _returnvalue_rotation) (`KismetMathLibrary.BreakTransform` (`SplineComponent.GetTransformAtDistanceAlongSpline` (`self.SplineComponent`) (`self.DistanceAlongSpline`) "World" false)))
  (switch `ECharacterType` (`self.CharacterType`)
    (:`Player`
      (bind _returnvalue (message `Speedable.GetCurrentSpeed` (`self.PlayerCharacter`)))
      (set `self.DistanceAlongSpline` (+ (* _returnvalue Delta) (`self.DistanceAlongSpline`))))
    (:`Enemy`
      (bind _returnvalue_2 (message `Speedable.GetCurrentSpeed` ActorToMove))
      (set `self.DistanceAlongSpline` (+ (* _returnvalue_2 Delta) (`self.DistanceAlongSpline`)))))
  (`self.K2_SetActorRelativeTransform` ActorToMove (`KismetMathLibrary.MakeTransform` _returnvalue_location _returnvalue_rotation) false false))

(fn `MoveEnemiesAlongSpline`
  (params (DeltaTime :type "Float (double-precision)"))
  (`self.MoveActorAlongSpline` (`self.EnemyParent`) DeltaTime))

(fn `MovePlayerAlongSpline`
  (params (DeltaTime :type "Float (double-precision)"))
  (`self.MoveActorAlongSpline` (`self.PlayerParent`) DeltaTime))

(fn `SetupEnemyGroup`
  (locals (Columns :type Integer64) (Rows :type Integer64) (OffsetY :type "Float (double-precision)"))
  (`KismetArrayLibrary.Array_Clear` (`self.EnemySpawnPonts`))
  (if (<= (`self.GroupSize`) 0)
    (return)
    (else
      (set `local.Columns` (`KismetMathLibrary.FCeil64` (`KismetMathLibrary.Sqrt` (`KismetMathLibrary.Conv_IntToDouble` (`self.GroupSize`)))))
      (set `local.Rows` (`KismetMathLibrary.FCeil64` (`KismetMathLibrary.Conv_Int64ToDouble` (/ (`self.GroupSize`) (`local.Columns`)))))
      (set `local.OffsetY` (`KismetMathLibrary.Conv_Int64ToDouble` (/ (* (- (`local.Columns`) 1) (`self.DistanceBetweenEnemies`)) 2)))
      (for _index (range (`self.GroupSize`))
        (bind _returnvalue (`AddComponent|NODE_AddStaticMeshComponent-3` :`RelativeTransform` (`KismetMathLibrary.MakeTransform` (`KismetMathLibrary.MakeVector` 0.0 (`KismetMathLibrary.Conv_Int64ToDouble` (- (* (/ _index (`local.Columns`)) (`self.DistanceBetweenEnemies`)) (`local.OffsetY`))) (`KismetMathLibrary.Conv_IntToDouble` (* (mod _index (`KismetMathLibrary.Conv_Int64ToInt` (`local.Columns`))) (`self.DistanceBetweenEnemies`)))) (struct) (2.0 2.0 2.0))))
        (`KismetArrayLibrary.Array_Add` (`self.EnemySpawnPonts`) _returnvalue)
        (`SceneComponent.K2_AttachToComponent` _returnvalue (`self.Root`) "None" "KeepRelative" "KeepRelative" "KeepRelative" false)
        (`SceneComponent.SetHiddenInGame` (`self.Root`) true true)))))

(fn `UserConstructionScript`
  (locals (`Loop Index` :type Integer))
  (switch `ECharacterType` (`self.CharacterType`)
    (:`Player`
      (`self.K2_SetActorTransform` (`self.PlayerParent`) (`SplineComponent.GetTransformAtSplinePoint` (`self.SplineComponent`) 0 "World" false) false false))
    (:`Enemy`
      (`self.SetupEnemyGroup`))))