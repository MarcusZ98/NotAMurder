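; Jellyfish actor that moves an animated mesh along a looping spline path, facing along it with a fixed rotation offset.
; Construction script applies two materials and places the mesh at its starting Distance.
; BeginPlay randomizes animation start position and scales travel and animation speeds by a master SpeedMultiplier.
; Tick adds Speed to Distance without delta time, so movement is frame-rate dependent, and resets Distance at the spline's end.
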(event `self.ReceiveBeginPlay`
  (`SkeletalMeshComponent.SetPosition` (`self.AnimMesh`) (`KismetMathLibrary.RandomFloatInRange` 0.0 3.333) true) ; Randomize Animation Starting Position
  (`PrimitiveComponent.SetMaterial` (`self.AnimMesh`) 0 (`self.Material_Element0`))
  (`PrimitiveComponent.SetMaterial` (`self.AnimMesh`) 1 (`self.Material_Element1`))
  ;[1 1 1] We multiply the 'AnimSpeed' and 'Speed' variables with the 'SpeedMultiplier' variable because we want the 'SpeedMultiplier' variable to be the master control over all speed variables.
  (set `self.AnimSpeed` (* (`self.SpeedMultiplier`) (`self.AnimSpeed`)))
  (set `self.Speed` (* (`self.SpeedMultiplier`) (`self.Speed`)))
  (`SkeletalMeshComponent.SetPlayRate` (`self.AnimMesh`) (`self.AnimSpeed`)) ; Set the AnimMesh's animation speed to be the 'AnimSpeed' variable's value
)

(event `self.ReceiveTick`
  (params (DeltaSeconds :type "Float (single-precision)"))
  ;[1 1 1] We check whether the "Distance" variable is greater than the total length of the spline, because if this is true, it means we should reset the "Distance" variable back to 0 to make it appear as if the mesh is looping around the spline
  (if (< (`self.Distance`) (`SplineComponent.GetSplineLength` (`self.Spline`)))
    ;[1 1 1] We increase the "Distance" variable by the "Speed" variable each tick because the AnimMesh uses the "Distance" variable to determine its position along the spline.  Continuously increasing it makes the AnimMesh 'travel' along the spline.
    (set `self.Distance` (+ (`self.Distance`) (`self.Speed`)))
    ;[1 1 1] We use the "Distance" variable to set the AnimMesh's position along the spline, and we set the AnimMesh's rotation to face forward along the spline because this will create the animation effect of the AnimMesh 'travelling" along the spline like a rollercoaster.
    (`SceneComponent.K2_SetWorldTransform` (`self.AnimMeshTransform`) (`KismetMathLibrary.MakeTransform` (`SplineComponent.GetLocationAtDistanceAlongSpline` (`self.Spline`) (`self.Distance`) "World") (`KismetMathLibrary.ComposeRotators` (`SplineComponent.GetRotationAtDistanceAlongSpline` (`self.Spline`) (`self.Distance`) "World") (struct :`Yaw` -90.0)) (`KismetMathLibrary.Conv_DoubleToVector` (`self.Scale`))) false false)
    (else
      (set `self.Distance` 0.0))))

(fn `UserConstructionScript`
  (`PrimitiveComponent.SetMaterial` (`self.AnimMesh`) 0 (`self.Material_Element0`))
  (`PrimitiveComponent.SetMaterial` (`self.AnimMesh`) 1 (`self.Material_Element1`))
  ;[1 1 1] We use the 'Distance' variable to set the AnimMesh's transform along the spline because we want to set the starting location of its animation along the spline.
  (`SceneComponent.K2_SetWorldTransform` (`self.AnimMeshTransform`) (`KismetMathLibrary.MakeTransform` (`SplineComponent.GetLocationAtDistanceAlongSpline` (`self.Spline`) (`self.Distance`) "World") (`KismetMathLibrary.ComposeRotators` (`SplineComponent.GetRotationAtDistanceAlongSpline` (`self.Spline`) (`self.Distance`) "World") (struct :`Yaw` -90.0)) (`KismetMathLibrary.Conv_DoubleToVector` (`self.Scale`))) false false))