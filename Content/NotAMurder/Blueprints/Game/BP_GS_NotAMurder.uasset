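; Game state for NotAMurder that tracks kills and total score and relays scoring events to the player HUD.
; Registered enemies have their kill and hit events bound here, adding points and updating the HUD score tracker, with hits also notifying the cursor widget.
; It also triggers the HUD win screen and holds the player spline reference, intended to be the only one.
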(event `self.ReceiveBeginPlay`
  (bind _asplayer_hud (cast `/Game/NotAMurder/Blueprints/Widgets/Player_HUD` (`PlayerController.GetHUD` (`GameplayStatics.GetPlayerController` 0)))
    (:`then`
      (set `self.Player HUD` _asplayer_hud))
    (:`CastFailed`
      (`KismetSystemLibrary.PrintString` "Failed cast to player HUD"))))

(event `RegisterEnemy`
  (params (Enemy :type "/Game/NotAMurder/Blueprints/Characters/Enemy/BP_EnemyCharacter Object Reference"))
  ;[1 0.2188 0.2188] Bind Enemy Events
  (add `/Game/NotAMurder/Blueprints/Characters/Enemy/BP_EnemyCharacter.OnEnemyKilled` Enemy (delegate `Killing Enemy`))
  (add `/Game/NotAMurder/Blueprints/Characters/Enemy/BP_EnemyCharacter.OnEnemyHit` Enemy (delegate `Hitting Enemy`)))

(event `Killing Enemy`
  (params (PointsWorth :type Integer))
  ;[1 0.6264 0.5565] On Enemy Killed
  (`/Engine/EditorBlueprintResources/StandardMacros.IncrementInt` (`self.NumberOfEnemiesKilled`)
    (:`  `
      (bind _output_get (set `self.TotalScore` (+ PointsWorth (`self.TotalScore`))))
      (`/Game/NotAMurder/Blueprints/Widgets/WB_ScoreTracker.Update Score` (`/Game/NotAMurder/Blueprints/Widgets/Player_HUD.ScoreTracker` (`self.Player HUD`)) PointsWorth _output_get))))

(event `Hitting Enemy`
  (params (PointsToAdd :type Integer))
  ;[1 0.6457 0.6556] On Enemy Hit
  (bind _output_get (set `self.TotalScore` (+ PointsToAdd (`self.TotalScore`))))
  (`/Game/NotAMurder/Blueprints/Widgets/WB_ScoreTracker.Update Score` (`/Game/NotAMurder/Blueprints/Widgets/Player_HUD.ScoreTracker` (`self.Player HUD`)) PointsToAdd _output_get)
  (`/Game/NotAMurder/Blueprints/Widgets/BP_Crosshair.OnEnemyHit` (`/Game/NotAMurder/Blueprints/Widgets/Player_HUD.CursorWidget` (`self.Player HUD`))))

(event `Show Win Screen`
  (`/Game/NotAMurder/Blueprints/Widgets/Player_HUD.Add Win Screen` (`self.Player HUD`)))

(event `Set Player Spline`
  (params (`Player Spline` :type "/Game/NotAMurder/Blueprints/Objects/Spline/BP_SplinePath Object Reference"))
  ;[1 1 1] Setup Player Spline REF
  (`/Engine/EditorBlueprintResources/StandardMacros.IsValid` (`self.Player Spline`)
    (:`Is Valid`
      (`KismetSystemLibrary.PrintString` "Can only have one player spline"))
    (:`Is Not Valid`
      (set `self.Player Spline` `Player Spline`))))

(fn `UserConstructionScript`)