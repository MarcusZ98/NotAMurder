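; Base weapon Blueprint that fires projectiles for player and enemy characters, with a cooldown between shots.
; FireWeapon spawns the WeaponData projectile along the aim vector, with the shooter as instigator, and assigns the hit target as homing component.
; Enemy shots explicitly enable homing and set its acceleration, while player shots leave both to the projectile's own settings.
; A successful shot clears the can-fire flag until a timer based on the weapon's fire rate resets it.
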(event `WeaponInterface.FireWeapon`
  (params (OwnerOfWeapon :type "BaseCharacter Object Reference") (StartLocation :type "Vector Structure (by ref)") (ForwardVector :type "Vector Structure (by ref)") (HitTarget :type "SceneComponent Object Reference"))
  (bind (_weapondata_damagepershot _weapondata_firerate _weapondata_projectile) (break `WeaponData` (`self.WeaponData`)))
  (bind (_weapondata_damagepershot_2 _weapondata_firerate_2) (break `WeaponData` (`self.WeaponData`)))
  (bind (_weapondata_damagepershot_3 _weapondata_firerate_3 _weapondata_projectile_2) (break `WeaponData` (`self.WeaponData`)))
  (bind (_weapondata_damagepershot_4 _weapondata_firerate_4) (break `WeaponData` (`self.WeaponData`)))
  (if (`self.BCanFire`)
    (bind _returnvalue (message `Character_Interface.GetCharacterType` OwnerOfWeapon))
    (switch `ECharacterType` _returnvalue
      (:`Player`
        (bind _returnvalue_2 (`|SpawnActorFromClass` _weapondata_projectile_2 (`KismetMathLibrary.MakeTransform` StartLocation (`KismetMathLibrary.Conv_VectorToRotator` ForwardVector)) "AlwaysSpawn" "MultiplyWithRoot" self OwnerOfWeapon))
        (`/Engine/EditorBlueprintResources/StandardMacros.IsValid` _returnvalue_2
          (:`Is Valid`
            (bind _asbp_base_projectile (cast `/Game/NotAMurder/Blueprints/Objects/Weapons/BP_BaseProjectile` _returnvalue_2))
            (bind _projectilemovement (`/Game/NotAMurder/Blueprints/Objects/Weapons/BP_BaseProjectile.ProjectileMovement` _asbp_base_projectile)
              (:`then`
                (set `ProjectileMovementComponent.HomingTargetComponent` HitTarget _projectilemovement)
                (set `self.BCanFire` false)
                (`KismetSystemLibrary.K2_SetTimer` null "ResetFireFlag" _weapondata_firerate_4))
              (:`else`)))))
      (:`Enemy`
        (bind _returnvalue_3 (`|SpawnActorFromClass` _weapondata_projectile (`KismetMathLibrary.MakeTransform` StartLocation (`KismetMathLibrary.Conv_VectorToRotator` ForwardVector)) "AlwaysSpawn" "MultiplyWithRoot" self OwnerOfWeapon))
        (`/Engine/EditorBlueprintResources/StandardMacros.IsValid` _returnvalue_3
          (:`Is Valid`
            (bind _asbp_base_projectile_2 (cast `/Game/NotAMurder/Blueprints/Objects/Weapons/BP_BaseProjectile` _returnvalue_3))
            (bind _projectilemovement_2 (`/Game/NotAMurder/Blueprints/Objects/Weapons/BP_BaseProjectile.ProjectileMovement` _asbp_base_projectile_2)
              (:`then`
                (set `ProjectileMovementComponent.bIsHomingProjectile` true _projectilemovement_2)
                (set `ProjectileMovementComponent.HomingTargetComponent` HitTarget _projectilemovement_2)
                (set `ProjectileMovementComponent.HomingAccelerationMagnitude` 3000.0 _projectilemovement_2)
                (set `self.BCanFire` false)
                (`KismetSystemLibrary.K2_SetTimer` null "ResetFireFlag" _weapondata_firerate_2))
              (:`else`))))))))

(fn `ResetFireFlag`
  (set `self.BCanFire` true))

(fn `UserConstructionScript`)