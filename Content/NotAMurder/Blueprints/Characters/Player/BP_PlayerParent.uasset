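; Player base Blueprint that acts as the view target, with a mouse-steered camera and an input-driven child actor.
; On Tick, the cursor leaving a central dead zone turns the camera within tight clamps, interpolating faster the farther it is from screen center.
; IA_Move slides the child actor along local Y and Z toward clamped limits.
; MoveChildrenLocal is a stub, and the deproject-based camera move is disconnected.
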(event `self.ReceiveBeginPlay`
  ;[1 1 1] Sets this camera as view
  (`PlayerController.SetViewTargetWithBlend` (`GameplayStatics.GetPlayerController` 0) self 0.0 "VTBlend_Linear" 0.0 false))

(event `self.ReceiveTick`
  (params (DeltaSeconds :type "Float (single-precision)"))
  (bind (_returnvalue_x _returnvalue_y) (`KismetMathLibrary.BreakVector2D` (`WidgetLayoutLibrary.GetViewportSize`)))
  (bind (_returnvalue_x_2 _returnvalue_y_2) (`KismetMathLibrary.BreakVector2D` (`|GetInputActionValue`)))
  (bind (_locationx _locationy) (`PlayerController.GetMousePosition` (`GameplayStatics.GetPlayerController` 0)))
  (bind (_locationx_2 _locationy_2) (`PlayerController.GetMousePosition` (`GameplayStatics.GetPlayerController` 0)))
  (bind (_returnvalue_x_3 _returnvalue_y_3) (`KismetMathLibrary.BreakVector2D` (/ (`WidgetLayoutLibrary.GetViewportSize`) (2.0 2.0))))
  (bind (_relativerotation_roll _relativerotation_pitch _relativerotation_yaw) (`KismetMathLibrary.BreakRotator` (`SceneComponent.RelativeRotation` (`self.Camera`))))
  (bind (_relativerotation_roll_2 _relativerotation_pitch_2 _relativerotation_yaw_2) (`KismetMathLibrary.BreakRotator` (`SceneComponent.RelativeRotation` (`self.Camera`))))
  (bind (_relativelocation_x _relativelocation_y _relativelocation_z) (`KismetMathLibrary.BreakVector` (`SceneComponent.RelativeLocation` (`self.ChildActor`))))
  (bind _relativelocation_x_2 (`KismetMathLibrary.BreakVector` (`SceneComponent.RelativeLocation` (`self.ChildActor`))))
  (bind _returnvalue (- _locationx (/ _returnvalue_x 2.0)))
  (bind _returnvalue_2 (- (/ _returnvalue_y 2.0) _locationy))
  (bind (_returnvalue_roll _returnvalue_pitch _returnvalue_yaw) (`KismetMathLibrary.BreakRotator` (`KismetMathLibrary.RInterpTo` (`SceneComponent.RelativeRotation` (`self.Camera`)) (`KismetMathLibrary.MakeRotator` _relativerotation_roll_2 (`self.NewPitchValue`) (`self.NewYawValue`)) (* DeltaSeconds (`KismetMathLibrary.Lerp` 0.0 0.5 (`self.RotationForceNew`))) 2.0)))
  (bind (_returnvalue_x_4 _returnvalue_y_4 _returnvalue_z) (`KismetMathLibrary.BreakVector` (`KismetMathLibrary.VLerp` (`SceneComponent.RelativeLocation` (`self.ChildActor`)) (`KismetMathLibrary.MakeVector` _relativelocation_x_2 (`KismetMathLibrary.FClamp` (+ (* _returnvalue_x_2 500.0) _relativelocation_y) (`self.PlayerPositionMinLimitX`) (`self.PlayerPositionMaxLimitX`)) (`KismetMathLibrary.FClamp` (+ _relativelocation_z (* _returnvalue_y_2 500.0)) (`self.PlayerPositionMinLimitY`) (`self.PlayerPositionMaxLimitY`))) (* DeltaSeconds 0.8))))
  ;[1 1 1] Tick
  (`|ExecutionSequence`
    (:`then_0`
      ;;[1 1 1] Sets a new target rotation if cursor is outside the horizontal limits
      (if (> (`KismetMathLibrary.Abs` _returnvalue) (`self.HorizontalMinLimit`))
        (set `self.NewYawValue` (+ (* (`KismetMathLibrary.SignOfFloat` _returnvalue) 100.0) _relativerotation_yaw))
        (else
          (set `self.NewYawValue` _relativerotation_yaw_2))))
    (:`then_1`
      ;;[1 1 1] Sets a new target rotation if cursor is outside the vertical limits
      (if (> (`KismetMathLibrary.Abs` _returnvalue_2) (`self.VerticalMinLimit`))
        (set `self.NewPitchValue` (+ _relativerotation_pitch (* (`KismetMathLibrary.SignOfFloat` _returnvalue_2) 100.0)))
        (else
          (set `self.NewPitchValue` _relativerotation_pitch_2))))
    (:`then_2`
      (set `self.RotationForceNew` (/ (`KismetMathLibrary.Distance2D` (`KismetMathLibrary.MakeVector2D` _returnvalue_x_3 _returnvalue_y_3) (`KismetMathLibrary.MakeVector2D` _locationx_2 _locationy_2)) (`KismetMathLibrary.VSize2D` (`KismetMathLibrary.MakeVector2D` _returnvalue_x_3 _returnvalue_y_3)))))
    (:`then_3`
      ;;[1 1 1] Makes a new target rotator, and sets it under time.
      (`SceneComponent.K2_SetRelativeRotation` (`self.Camera`) (`KismetMathLibrary.MakeRotator` (`KismetMathLibrary.FClamp` _returnvalue_roll -5.0 5.0) (`KismetMathLibrary.FClamp` _returnvalue_pitch -10.0 10.0) (`KismetMathLibrary.FClamp` _returnvalue_yaw -10.0 10.0)) false false))
    (:`then_4`
      ;;[1 1 1] Moves the actor child localy in only two axis
      (`SceneComponent.K2_SetRelativeLocation` (`self.ChildActor`) (`KismetMathLibrary.MakeVector` _returnvalue_x_4 _returnvalue_y_4 _returnvalue_z) false false))))

(fn `MoveChildrenLocal`
  (params (NewY :type "Float (double-precision)") (DeltaTime :type "Float (double-precision)"))
  (returns (newYValue :type "Float (double-precision)"))
  (return 0.0))

(fn `UserConstructionScript`)