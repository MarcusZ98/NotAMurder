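; Enemy character in a game with a spline-following player: it registers with the game state and stays hidden until StartEnemy.
; Once started, it faces the player and, if armed, attempts fire on a randomly offset looping timer while ahead along the spline.
; Shots lead the player by solving a quadratic intercept from spline velocity and projectile speed.
; Damage triggers hit and kill scoring calls and an explosion on death; dummies ignore damage and leave the enemy count.
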(event `self.ReceiveBeginPlay`
  (`SceneComponent.SetHiddenInGame` (`self.Mesh`) true false)
  (set `self.Player` (`GameplayStatics.GetPlayerCharacter` 0))
  (bind _asbp_gs_not_amurder (cast `/Game/NotAMurder/Blueprints/Game/BP_GS_NotAMurder` (`GameplayStatics.GetGameState`)))
  (`/Game/NotAMurder/Blueprints/Game/BP_GS_NotAMurder.RegisterEnemy` _asbp_gs_not_amurder self)
  (bind _returnvalue (`PrimitiveComponent.CreateDynamicMaterialInstance` (`self.Mesh`) 0 null "None"))
  (set `self.DynamicMaterial` _returnvalue)
  (`KismetSystemLibrary.DelayUntilNextTick`)
  (setmembers `CharacterData` :`StructRef` (`self.CharacterData`) :`CurrentHealth` (`.MaxHealth` (break `CharacterData` (`self.CharacterData`)))))

(event `Make Dummy`
  ;[1 1 1] Make Dummy
  (set `self.bIsDummy?` true)
  (bind _asbp_gs_not_amurder (cast `/Game/NotAMurder/Blueprints/Game/BP_GS_NotAMurder` (`GameplayStatics.GetGameState`)))
  (bind _result (`/Engine/EditorBlueprintResources/StandardMacros.DecrementInt` (`/Game/NotAMurder/Blueprints/Game/BP_GS_NotAMurder.TotalNumberOfEnemies` _asbp_gs_not_amurder))
    (:`  `
      (set `/Game/NotAMurder/Blueprints/Game/BP_GS_NotAMurder.TotalNumberOfEnemies` _result _asbp_gs_not_amurder))))

(event `Start Enemy`
  ;[0.94 1 0.5744] Auto Fire
  (`|ExecutionSequence`
    (:`then_0`
      (`self.SetActorTickEnabled` true)
      (`SceneComponent.SetHiddenInGame` (`self.Mesh`) false false))
    (:`then_1`
      (`KismetSystemLibrary.Delay` (`KismetMathLibrary.RandomFloatInRange` 0.0 1.0))
      (`/Engine/EditorBlueprintResources/StandardMacros.IsValid` (`.WeaponInstance` (break `CharacterData` (`self.CharacterData`)))
        (:`Is Valid`
          (`KismetSystemLibrary.K2_SetTimerDelegate` (delegate `Fire`) 0.1 true))))))

(event `self.ReceiveAnyDamage`
  (params (Damage :type "Float (single-precision)") (DamageType :type "DamageType Object Reference") (InstigatedBy :type "Controller Object Reference") (DamageCauser :type "Actor Object Reference"))
  ;[1 0.5611 0.5412] Take Damage
  (if (not (`self.bIsDummy?`))
    (setmembers `CharacterData` :`StructRef` (`self.CharacterData`) :`CurrentHealth` (- (`.CurrentHealth` (break `CharacterData` (`self.CharacterData`))) Damage))
    (`self.OnEnemyHit` (`self.Points to Add Per Hit`))
    (if (`self.Is HP below 0?`)
      (`self.DestroyActor`))))

(event `Fire`
  (bind (_characterdata_maxhealth _characterdata_currenthealth _characterdata_movementspeed _characterdata_charactertype _characterdata_weapon _characterdata_weaponinstance) (break `CharacterData` (`self.CharacterData`)))
  (bind (_weapondata_damagepershot _weapondata_firerate _weapondata_projectile _weapondata_projectilespeed) (break `WeaponData` (`BaseWeapon.WeaponData` _characterdata_weaponinstance)))
  ;[0.94 1 0.5744] Auto Fire
  (bind _result (`self.IsInFrontOfPLayer?`))
  (if _result
    (bind _asbp_gs_not_amurder (cast `/Game/NotAMurder/Blueprints/Game/BP_GS_NotAMurder` (`GameplayStatics.GetGameState`)))
    (bind (_result_2 _check) (`self.InterceptionDirection` (`self.K2_GetActorLocation` (`GameplayStatics.GetPlayerCharacter` 0)) (`self.K2_GetActorLocation`) (`/Game/NotAMurder/Blueprints/Objects/Spline/BP_SplinePath.PlayerVelocity` (`/Game/NotAMurder/Blueprints/Game/BP_GS_NotAMurder.Player Spline` _asbp_gs_not_amurder)) _weapondata_projectilespeed))
    (if _check
      (message `WeaponInterface.FireWeapon` (`.WeaponInstance` (break `CharacterData` (`self.CharacterData`))) self (`SceneComponent.K2_GetComponentLocation` (`self.ShootStartLocation`)) _result_2 (`Actor.RootComponent` (`self.Player`)))
      (else
        (`KismetSystemLibrary.PrintString` "Will not hit player")))))

(event `self.ReceiveTick`
  (params (DeltaSeconds :type "Float (single-precision)"))
  ;[0.7081 1 0.7316] Make Enemy look at Player
  (if (`self.bLookAtPlayer?`)
    (`self.K2_SetActorRotation` (`KismetMathLibrary.FindLookAtRotation` (`self.K2_GetActorLocation`) (`self.K2_GetActorLocation` (`self.Player`))))))

(fn `CalculateQuadraticEquation`
  (params (A :type "Float (double-precision)") (B :type "Float (double-precision)") (C :type "Float (double-precision)"))
  (returns (Root1 :type "Float (double-precision)") (Root2 :type "Float (double-precision)") (Check :type "Float (double-precision)"))
  (locals (Discriminant :type "Float (double-precision)") (RootOne :type "Float (double-precision)") (RootTwo :type "Float (double-precision)"))
  (bind _output_get (set `local.Discriminant` (- (`KismetMathLibrary.Square` (`local.B`)) (* (`local.A`) (`local.C`) 4.0))))
  ;[1 1 1] If less than zero we have no valid answer
  (if (< _output_get 0.0)
    (set `local.RootOne` 0.0)
    (set `local.RootTwo` 0.0)
    (return 0.0 0.0 0.0)
    (else
      (set `local.RootOne` (/ (+ (* (`local.B`) -1.0) (`KismetMathLibrary.Sqrt` (`local.Discriminant`))) (* (`local.A`) 2.0)))
      (set `local.RootTwo` (/ (- (* (`local.B`) -1.0) (`KismetMathLibrary.Sqrt` (`local.Discriminant`))) (* (`local.A`) 2.0)))
      (return (`local.RootOne`) (`local.RootTwo`) (`KismetMathLibrary.SelectFloat` 2.0 1.0 (> (`local.Discriminant`) 0.0))))))

(fn `DestroyActor`
  (`NiagaraFunctionLibrary.SpawnSystemAtLocation` "/Game/ProjectileHitVFX/NS/NS_HIt_Explosion.NS_HIt_Explosion" (`SceneComponent.K2_GetComponentLocation` (`self.Mesh`)))
  (`self.OnEnemyKilled` (`.PointsWorth` (break `EnemyData` (`self.EnemyData`))))
  (`Enemy_Interface.KillEnemy`))

(fn `EnemyHit`)

(fn `GetShootDirection`
  (returns (`Shoot Direction` :type "Vector Structure"))
  (bind _asbp_gs_not_amurder (cast `/Game/NotAMurder/Blueprints/Game/BP_GS_NotAMurder` (`GameplayStatics.GetGameState`)))
  (return (`KismetMathLibrary.Conv_RotatorToVector` (`KismetMathLibrary.FindLookAtRotation` (`self.K2_GetActorLocation`) (`self.K2_GetActorLocation` (`self.Player`))))))

(fn `InterceptionDirection`
  (params (a :type "Vector Structure") (b :type "Vector Structure") (vA :type "Vector Structure") (sB :type "Float (double-precision)"))
  (returns (Result :type "Vector Structure") (Check :type Boolean))
  (locals (aToB :type "Vector Structure") (dC :type "Float (double-precision)") (Alpha :type "Float (double-precision)") (SA :type "Float (double-precision)") (r :type "Float (double-precision)") (dA :type "Float (double-precision)") (t :type "Float (double-precision)") (C :type "Vector Structure"))
  (set `local.aToB` (- (`local.b`) (`local.a`)))
  (set `local.dC` (`KismetMathLibrary.VSize` (`local.aToB`)))
  (set `local.Alpha` (`KismetMathLibrary.DegreesToRadians` (`KismetMathLibrary.Vector_CosineAngle2D` (`local.aToB`) (`local.vA`))))
  (set `local.SA` (`KismetMathLibrary.VSize` (`local.vA`)))
  (set `local.r` (/ (`local.SA`) (`local.sB`)))
  (bind (_root1 _root2 _check) (`self.CalculateQuadraticEquation` (- 1.0 (`KismetMathLibrary.Square` (`local.r`))) (* (`local.r`) (`KismetMathLibrary.Cos` (`local.Alpha`)) (`local.dC`) 2.0) (* (`KismetMathLibrary.Square` (`local.dC`)) -1.0)))
  (if (== _check 0.0)
    (return (`KismetMathLibrary.Vector_Zero`) false)
    (else
      (set `local.dA` (`KismetMathLibrary.FMax` _root1 _root2))
      (set `local.t` (/ (`local.dA`) (`local.sB`)))
      (set `local.C` (+ (* (`local.vA`) (`local.t`)) (`local.a`)))
      (return (`KismetMathLibrary.Normal` (- (`local.C`) (`local.b`))) true))))

(fn `IsInFrontOfPLayer?`
  (returns (Result :type Boolean))
  (bind _asbp_gs_not_amurder (cast `/Game/NotAMurder/Blueprints/Game/BP_GS_NotAMurder` (`GameplayStatics.GetGameState`)))
  (bind _player_spline (`/Game/NotAMurder/Blueprints/Game/BP_GS_NotAMurder.Player Spline` _asbp_gs_not_amurder))
  (`/Engine/EditorBlueprintResources/StandardMacros.IsValid` _player_spline
    (:`Is Valid`
      (return (> (`KismetMathLibrary.Dot_VectorVector` (`KismetMathLibrary.Normal` (`SplineComponent.GetTangentAtDistanceAlongSpline` (`SplinePath.SplineComponent` _player_spline) (`SplinePath.CurrentDistanceAlongSpline` _player_spline) "World")) (`KismetMathLibrary.Normal` (- (`self.K2_GetActorLocation`) (`self.K2_GetActorLocation` (`self.Player`))))) 0.0)))))

(fn `UserConstructionScript`)