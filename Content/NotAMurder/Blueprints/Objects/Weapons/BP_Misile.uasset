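; BP_Misile is an explosive missile projectile that deals area damage on contact.
; When its sphere begins overlapping an actor that passes IsDifferentCharacter, it spawns the impact effect from ProjectileData at the hit point.
; It then applies full, non-falloff radial damage, sized by HowMuchDamageToDeal from its instigator, ignoring itself, and destroys itself.
; A debug-sphere draw is left unconnected.
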(event `self.ReceiveBeginPlay`
  (`parent.ReceiveBeginPlay`))

(event `self.Sphere.OnComponentBeginOverlap`
  (params (OverlappedComponent :type "PrimitiveComponent Object Reference") (OtherActor :type "Actor Object Reference") (OtherComp :type "PrimitiveComponent Object Reference") (OtherBodyIndex :type Integer) (bFromSweep :type Boolean) (SweepResult :type "HitResult Structure (by ref)"))
  (bind (_projectiledata_projectilefx _projectiledata_impactfx) (break `ProjectileData` (`self.ProjectileData`)))
  (bind _result (`self.IsDifferentCharacter?` OtherActor))
  (if _result
    (bind _damage (`self.HowMuchDamageToDeal?` (`self.GetInstigator`)))
    (`NiagaraFunctionLibrary.SpawnSystemAtLocation` _projectiledata_impactfx SweepResult_ImpactPoint)
    (`GameplayStatics.ApplyRadialDamage` _damage SweepResult_Location 600.0 null (`|MakeArray` self :!type "Actor Object Reference") null null true "ECC_WorldStatic")
    (`self.K2_DestroyActor`)))

(fn `UserConstructionScript`
  (`parent.UserConstructionScript`))