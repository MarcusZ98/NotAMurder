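; Spline path actor that moves either the player or an enemy group along its spline, set by CharacterType.
; Construction lays out hidden mesh markers from saved positions or a computed grid, where enemies spawn attached to a hidden dummy leader.
; Tick advances distance by the mover's speed and tracks player velocity.
; The player reaching the end shows the win screen, while enemy groups destroy their members and the spline.
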(event `Stop Spline`
  (`self.SetActorTickEnabled` false))

(event `Start Spline`
  (`self.SetActorTickEnabled` true)
  (for _array_element (`self.EnemyCharacters`)
    (`/Engine/EditorBlueprintResources/StandardMacros.IsValid` _array_element
      (:`Is Valid`
        (bind _asbp_enemy_character (cast `/Game/NotAMurder/Blueprints/Characters/Enemy/BP_EnemyCharacter` _array_element))
        (`/Game/NotAMurder/Blueprints/Characters/Enemy/BP_EnemyCharacter.Start Enemy` _asbp_enemy_character)))))

(event `self.ReceiveBeginPlay`
  (switch `ECharacterType` (`self.CharacterType`)
    (:`Player`
      (`self.AttachPlayerToSpline`)
      (`self.Start Spline`)
      (bind _asbp_gs_not_amurder (cast `/Game/NotAMurder/Blueprints/Game/BP_GS_NotAMurder` (`GameplayStatics.GetGameState`)))
      (`/Game/NotAMurder/Blueprints/Game/BP_GS_NotAMurder.Set Player Spline` _asbp_gs_not_amurder self)
      (set `self.PreviousPosition` (`self.K2_GetActorLocation` (`self.PlayerCharacter`))))
    (:`Enemy`
      (`self.AttachEnemyToSpline`))))

(event `self.ReceiveTick`
  (params (DeltaSeconds :type "Float (single-precision)"))
  (switch `ECharacterType` (`self.CharacterType`)
    (:`Player`
      (`self.MovePlayerAlongSpline` DeltaSeconds)
      ;[1 1 1] Calculates player velocity
      (set `self.currentPosition` (`self.K2_GetActorLocation` (`self.PlayerCharacter`)))
      (bind _output_get (set `self.PlayerVelocity` (/ (- (`self.currentPosition`) (`self.PreviousPosition`)) DeltaSeconds)))
      (set `self.PreviousPosition` (`self.currentPosition`))
      (`KismetSystemLibrary.PrintString` (`KismetStringLibrary.Conv_VectorToString` _output_get)))
    (:`Enemy`
      (`self.MoveEnemiesAlongSpline` DeltaSeconds))))

(fn `AttachEnemyToSpline`
  (bind _returnvalue (`|SpawnActorFromClass` (`self.EnemyClass`) (`SplineComponent.GetTransformAtSplinePoint` (`self.SplineComponent`) 0 "World" false) "AlwaysSpawn" "MultiplyWithRoot" null null))
  (bind _output_get (set `self.EnemyParent` _returnvalue))
  (if (`self.bOverrideCharacterData`)
    (message `Character_Interface.SetCharacterData` _output_get (`self.OverridenCharacterData`))
    (if (`self.bOverrideEnemyData`)
      (message `Enemy_Interface.SetEnemyData` _output_get (`self.OverriddenEnemyData`))))
  (`self.SetActorHiddenInGame` _output_get true)
  (bind _asbp_enemy_character (cast `/Game/NotAMurder/Blueprints/Characters/Enemy/BP_EnemyCharacter` _output_get))
  (`/Game/NotAMurder/Blueprints/Characters/Enemy/BP_EnemyCharacter.Make Dummy` _asbp_enemy_character)
  (`PrimitiveComponent.SetCollisionObjectType` (`Character.CapsuleComponent` _asbp_enemy_character) "ECC_Vehicle")
  (for _array_element (`self.EnemySpawningPositions`)
    (bind _returnvalue_2 (`|SpawnActorFromClass` (`self.EnemyClass`) (`SceneComponent.K2_GetComponentToWorld` _array_element) "AlwaysSpawn" "MultiplyWithRoot" null null))
    (`KismetArrayLibrary.Array_Add` (`self.EnemyCharacters`) _returnvalue_2)
    (if (`self.bOverrideEnemyData`)
      (message `Enemy_Interface.SetEnemyData` _returnvalue_2 (`self.OverriddenEnemyData`))
      (if (`self.bOverrideCharacterData`)
        (message `Character_Interface.SetCharacterData` _returnvalue_2 (`self.OverridenCharacterData`))))
    (`self.K2_AttachToActor` _returnvalue_2 (`self.EnemyParent`) "None" "KeepWorld" "KeepRelative" "KeepRelative" false))
  (return))

(fn `AttachPlayerToSpline`
  (bind _asbp_player_parent_1 (cast `/Game/NotAMurder/Blueprints/Characters/Player/BP_PlayerParent1` (`self.PlayerParent`)))
  (bind _asbp_player (cast `/Game/NotAMurder/Blueprints/Characters/Player/BP_Player` (`ChildActorComponent.ChildActor` (`/Game/NotAMurder/Blueprints/Characters/Player/BP_PlayerParent1.ChildActor` _asbp_player_parent_1))))
  (set `self.PlayerCharacter` _asbp_player)
  (if (not (`self.bOverrideCharacterData`))
    (`self.K2_SetActorTransform` (`self.PlayerParent`) (`SplineComponent.GetTransformAtSplinePoint` (`self.SplineComponent`) 0 "World" false) false false)
    (set `self.CurrentDistanceAlongSpline` (`SplineComponent.GetDistanceAlongSplineAtSplinePoint` (`self.SplineComponent`) (`self.SpawnIndex`)))))

(fn `GetPlayertLocation`
  (params (TimeToImpact :type "Float (double-precision)"))
  (returns (FuturePlayerLocation :type "Vector Structure"))
  ;[1 1 1] Old
  (bind _returnvalue (`Speedable.GetCurrentSpeed` (`self.PlayerCharacter`)))
  (return (`SplineComponent.GetLocationAtDistanceAlongSpline` (`self.SplineComponent`) (+ (* _returnvalue TimeToImpact) (`SplineComponent.GetDistanceAlongSplineAtLocation` (`self.SplineComponent`) (`self.K2_GetActorLocation` (`self.PlayerParent`)) "Local") 500.0) "World")))

(fn `GetPlayerVelocity`
  (returns (Velocity :type "Vector Structure"))
  ;[1 1 1] New
  (return (`self.PlayerVelocity`)))

(fn `MoveActorAlongSpline`
  (params (ActorToMove :type "Actor Object Reference") (Delta :type "Float (double-precision)"))
  (bind (_returnvalue_location _returnvalue_rotation) (`KismetMathLibrary.BreakTransform` (`SplineComponent.GetTransformAtDistanceAlongSpline` (`self.SplineComponent`) (`self.CurrentDistanceAlongSpline`) "World" false)))
  (switch `ECharacterType` (`self.CharacterType`)
    (:`Player`
      (bind _returnvalue (message `Speedable.GetCurrentSpeed` (`self.PlayerCharacter`)))
      (set `self.CurrentDistanceAlongSpline` (+ (* _returnvalue Delta) (`self.CurrentDistanceAlongSpline`)))
      (`self.K2_SetActorRelativeRotation` ActorToMove _returnvalue_rotation false false))
    (:`Enemy`
      (bind _returnvalue_2 (message `Speedable.GetCurrentSpeed` ActorToMove))
      (set `self.CurrentDistanceAlongSpline` (+ (* _returnvalue_2 Delta) (`self.CurrentDistanceAlongSpline`)))))
  (`self.K2_SetActorRelativeLocation` ActorToMove _returnvalue_location false false)
  (if (>= (`self.CurrentDistanceAlongSpline`) (`self.TotalSplineLength`))
    (switch `ECharacterType` (`self.CharacterType`)
      (:`Player`
        (bind _asbp_gs_not_amurder (cast `/Game/NotAMurder/Blueprints/Game/BP_GS_NotAMurder` (`GameplayStatics.GetGameState`)))
        (`/Game/NotAMurder/Blueprints/Game/BP_GS_NotAMurder.Show Win Screen` _asbp_gs_not_amurder))
      (:`Enemy`
        (for _array_element (`self.EnemyCharacters`)
          (`/Engine/EditorBlueprintResources/StandardMacros.IsValid` _array_element
            (:`Is Valid`
              (`self.K2_DestroyActor` _array_element))))
        (`self.K2_DestroyActor`)))))

(fn `MoveEnemiesAlongSpline`
  (params (DeltaTime :type "Float (double-precision)"))
  (`self.MoveActorAlongSpline` (`self.EnemyParent`) DeltaTime))

(fn `MovePlayerAlongSpline`
  (params (DeltaTime :type "Float (double-precision)"))
  (`self.MoveActorAlongSpline` (`self.PlayerParent`) DeltaTime))

(fn `SetupEnemyGroup`
  (locals (Columns :type Integer64) (Rows :type Integer64) (OffsetY :type "Float (double-precision)"))
  (`KismetArrayLibrary.Array_Clear` (`self.EnemySpawningPositions`))
  (if (== (`self.GroupSize`) (`KismetArrayLibrary.Array_Length` (`self.SavedEnemyPositions`)))
    (for _array_element (`self.SavedEnemyPositions`)
      (bind _returnvalue (`AddComponent|NODE_AddStaticMeshComponent-4` :`RelativeTransform` (`KismetMathLibrary.MakeTransform` _array_element (struct) (2.0 2.0 2.0))))
      (`KismetArrayLibrary.Array_Add` (`self.EnemySpawningPositions`) _returnvalue)
      (`SceneComponent.K2_AttachToComponent` _returnvalue (`self.Root`) "None" "KeepRelative" "KeepRelative" "KeepRelative" false)
      (`SceneComponent.SetHiddenInGame` (`self.Root`) true true)
      (`PrimitiveComponent.SetCollisionEnabled` _returnvalue "NoCollision"))
    (else
      (set `local.Columns` (`KismetMathLibrary.FCeil64` (`KismetMathLibrary.Sqrt` (`KismetMathLibrary.Conv_IntToDouble` (`self.GroupSize`)))))
      (set `local.Rows` (`KismetMathLibrary.FCeil64` (`KismetMathLibrary.Conv_Int64ToDouble` (/ (`self.GroupSize`) (`local.Columns`)))))
      (set `local.OffsetY` (`KismetMathLibrary.Conv_Int64ToDouble` (/ (* (- (`local.Columns`) 1) (`self.DistanceBetweenEnemies`)) 2)))
      (for _index (range (`self.GroupSize`))
        (bind _returnvalue_2 (`AddComponent|NODE_AddStaticMeshComponent-3` :`RelativeTransform` (`KismetMathLibrary.MakeTransform` (`KismetMathLibrary.MakeVector` 0.0 (`KismetMathLibrary.Conv_Int64ToDouble` (- (* (/ _index (`local.Columns`)) (`self.DistanceBetweenEnemies`)) (`local.OffsetY`))) (`KismetMathLibrary.Conv_IntToDouble` (* (mod _index (`KismetMathLibrary.Conv_Int64ToInt` (`local.Columns`))) (`self.DistanceBetweenEnemies`)))) (struct) (2.0 2.0 2.0))))
        (`KismetArrayLibrary.Array_Add` (`self.EnemySpawningPositions`) _returnvalue_2)
        (`SceneComponent.K2_AttachToComponent` _returnvalue_2 (`self.Root`) "None" "KeepRelative" "KeepRelative" "KeepRelative" false)
        (`SceneComponent.SetHiddenInGame` (`self.Root`) true true)
        (`PrimitiveComponent.SetCollisionEnabled` _returnvalue_2 "NoCollision")))))

(fn `UserConstructionScript`
  (locals (`Loop Index` :type Integer))
  (set `self.TotalSplineLength` (`SplineComponent.GetSplineLength` (`self.SplineComponent`)))
  (switch `ECharacterType` (`self.CharacterType`)
    (:`Player`
      (`self.K2_SetActorTransform` (`self.PlayerParent`) (`SplineComponent.GetTransformAtSplinePoint` (`self.SplineComponent`) (`self.SpawnIndex`) "World" false) false false))
    (:`Enemy`
      (`self.SetupEnemyGroup`))))