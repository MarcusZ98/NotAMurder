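; Base character Blueprint that implements Speedable events for changing a movement speed variable.
; The construction script caches MovementSpeed as OriginalMovementSpeed, which ResetSpeed restores.
; SetSpeed overwrites the current value and MultiplySpeed scales it, so repeated multipliers compound until a set or reset.
; GetSpeed returns the cached original speed, not the current one.
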(event `self.SetSpeed`
  (params (NewSpeed :type "Float (single-precision)"))
  ;[1 0.1875 0.1875] Speedable
  (set `self.MovementSpeed` NewSpeed))

(event `self.ResetSpeed`
  ;[1 0.1875 0.1875] Speedable
  (set `self.MovementSpeed` (`self.OriginalMovementSpeed`)))

(event `self.MultiplySpeed`
  (params (Multiplier :type "Float (single-precision)"))
  ;[1 0.1875 0.1875] Speedable
  (set `self.MovementSpeed` (* Multiplier (`self.MovementSpeed`))))

(fn `GetSpeed`
  (returns (ReturnValue :type "Float (single-precision)"))
  (return (`self.OriginalMovementSpeed`)))

(fn `UserConstructionScript`
  (set `self.OriginalMovementSpeed` (`self.MovementSpeed`)))