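; Trigger volume that changes the movement speed of overlapping characters whose type is in CharacterTypesToEffect, restoring it on exit.
; The target speed is NewMovementSpeed, optionally overwritten as a percentage of the character's original speed.
; Speed is set through message calls, either instantly or lerped by enter and exit timelines scaled to TransitionDuration.
; Exit stops the enter timeline and lerps from the target speed back to the original.
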(event `self.CollisionBox.OnComponentBeginOverlap`
  (params (OverlappedComponent :type "PrimitiveComponent Object Reference") (OtherActor :type "Actor Object Reference") (OtherComp :type "PrimitiveComponent Object Reference") (OtherBodyIndex :type Integer) (bFromSweep :type Boolean) (SweepResult :type "HitResult Structure (by ref)"))
  ;[0 1 0.07331] Begin Overlap
  (bind _result (`self.IsCharacterOfType?` OtherActor))
  (if _result
    (if (`self.bUsePercentageMovement`)
      (`self.ApplyPercentage` OtherActor))
    (if (`self.bUseSmoothTransition`)
      (`TimelineComponent.SetPlayRate` (`self.ChangeSpeedEnter`) (/ 1.0 (`self.TransitionDuration`)))
      (bind _returnvalue (message `Speedable.GetOriginalSpeed` OtherActor))
      (bind (_direction _alpha) (`Timeline|ChangeSpeedEnter` :!via `PlayFromStart`)
        (:`Update`
          (message `Speedable.SetCurrentSpeed` OtherActor (`KismetMathLibrary.Lerp` _returnvalue (`self.NewMovementSpeed`) _alpha)))
        (:`Finished`
          (`TimelineComponent.Stop` (`self.ChangeSpeedEnter`))))
      (else
        (message `Speedable.SetCurrentSpeed` OtherActor (`self.NewMovementSpeed`))))))

(event `self.CollisionBox.OnComponentEndOverlap`
  (params (OverlappedComponent :type "PrimitiveComponent Object Reference") (OtherActor :type "Actor Object Reference") (OtherComp :type "PrimitiveComponent Object Reference") (OtherBodyIndex :type Integer))
  ;[1 0 0] End Overlap
  (bind _result (`self.IsCharacterOfType?` OtherActor))
  (if _result
    (if (`self.bUseSmoothTransition`)
      (`TimelineComponent.Stop` (`self.ChangeSpeedEnter`))
      (`TimelineComponent.SetPlayRate` (`self.ChangeSpeedExit`) (/ 1.0 (`self.TransitionDuration`)))
      (bind _returnvalue (message `Speedable.GetOriginalSpeed` OtherActor))
      (bind (_direction _alpha) (`Timeline|ChangeSpeedExit` :!via `PlayFromStart`)
        (:`Update`
          (`/Engine/EditorBlueprintResources/StandardMacros.IsValid` OtherActor
            (:`Is Valid`
              (message `Speedable.SetCurrentSpeed` OtherActor (`KismetMathLibrary.Lerp` (`self.NewMovementSpeed`) _returnvalue _alpha)))))
        (:`Finished`
          (`TimelineComponent.Stop` (`self.ChangeSpeedExit`))))
      (else
        (message `Speedable.ResetSpeed` OtherActor)))))

(fn `ApplyPercentage`
  (params (OtherActor :type "Actor Object Reference"))
  (bind _returnvalue (message `Speedable.GetOriginalSpeed` OtherActor))
  (set `self.NewMovementSpeed` (* (/ _returnvalue 100.0) (`self.PercentageMovement`))))

(fn `IsCharacterOfType?`
  (params (Actor :type "Actor Object Reference"))
  (returns (Result :type Boolean))
  (bind _returnvalue (message `Character_Interface.GetCharacterData` Actor))
  (return (`KismetArrayLibrary.Array_Contains` (`self.CharacterTypesToEffect`) (`.CharacterType` (break `CharacterData` _returnvalue)))))

(fn `UserConstructionScript`)